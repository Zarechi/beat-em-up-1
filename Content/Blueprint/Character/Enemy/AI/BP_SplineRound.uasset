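; BP_SplineRound is a spline-based route for enemy AI that supplies world-space points, likely for patrol rounds.
; On BeginPlay it projects each spline point onto the navmesh within a search extent and caches the results in SplinePointLocation.
; GetSplinePoints exposes that cached array, while IncrementSplinePoint is a stub that returns a zero vector.
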(event `self.ReceiveBeginPlay`
  (for _index (range (`SplineComponent.GetNumberOfSplinePoints` (`self.Spline`)))
    (`KismetArrayLibrary.Array_Add` (`self.SplinePointLocation`) (`NavigationSystemV1.K2_ProjectPointToNavigation` (`SplineComponent.GetLocationAtSplinePoint` (`self.Spline`) _index "World") null null (500.0 500.0 500.0)))))

(fn `GetSplinePoints`
  (returns (SplinePoints :type "Array of Vector Structure"))
  (return (`self.SplinePointLocation`)))

(fn `IncrementSplinePoint`
  (returns (SplinePoint :type "Vector Structure"))
  (return (0.0 0.0 0.0)))

(fn `UserConstructionScript`)