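; Player character Blueprint that handles camera-relative movement, look, jump, sprint and a montage-based melee attack.
; Sprint sets walk speed from GetSprintSpeed, whose forward-motion speed selection is unconnected, and release restores MaxWalkSpeed.
; Attack picks a combo montage section by counter, but blocks input until completion resets that counter.
; A camera yaw clamp is present but never runs.
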(event `InputAxis|MoveForward`
  (params (AxisValue :type "Float (single-precision)"))
  (`self.AddMovementInput` (`SceneComponent.GetForwardVector` (`self.Camera`)) AxisValue))

(event `InputAxis|MoveRight`
  (params (AxisValue :type "Float (single-precision)"))
  (`self.AddMovementInput` (`SceneComponent.GetRightVector` (`self.Camera`)) AxisValue))

(event `InputAxis|LookUp`
  (params (AxisValue :type "Float (single-precision)"))
  (`self.AddControllerPitchInput` AxisValue))

(event `InputAxis|LookRight`
  (params (AxisValue :type "Float (single-precision)"))
  (`self.AddControllerYawInput` AxisValue))

(event `InputAction|Sprint`
  (params (Key :type "Key Structure"))
  (:`Pressed`
    (set `CharacterMovementComponent.MaxWalkSpeed` (`KismetMathLibrary.SelectFloat` (`self.MaxRunSpeed`) (`self.MaxWalkSpeed`) (> (`KismetMathLibrary.Dot_VectorVector` (`KismetMathLibrary.Normal` (`self.GetVelocity`)) (`self.GetActorForwardVector`)) 0.01)) (`self.CharacterMovement`)))
  (:`Released`
    (set `CharacterMovementComponent.MaxWalkSpeed` (`self.MaxWalkSpeed`) (`self.CharacterMovement`))))

(event `InputAction|Jump`
  (params (Key :type "Key Structure"))
  (:`Pressed`
    (`self.Jump`)))

(event `InputAction|Attack`
  (params (Key :type "Key Structure"))
  (:`Pressed`
    (if (not (`self.IsAttacking?`))
      (`|PlayMontage` (`self.Mesh`) "/Game/Animation/Warrok/Attack/Combo_Montage.Combo_Montage" 1.0 0.0 (select `int` (`self.AttackCtr`) :`0` "01" :`1` "02" :`2` "03" :!type "Name")
        (:`then`
          (set `self.IsAttacking?` true)
          (`/Engine/EditorBlueprintResources/StandardMacros.IncrementInt` (`self.AttackCtr`)))
        (:`OnCompleted`
          (set `self.IsAttacking?` false)
          (set `self.AttackCtr` 0))))))

(fn `UserConstructionScript`)