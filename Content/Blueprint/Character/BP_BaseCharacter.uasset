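; Base character Blueprint that gives characters hit points and a configurable walk speed.
; On BeginPlay it applies MaxWalkSpeed to the character movement component.
; Any damage subtracts from HP, and the actor destroys itself when HP reaches zero or below.
; Tick prints the actor's name and current HP on screen as a debug readout.
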(event `self.ReceiveBeginPlay`
  (set `CharacterMovementComponent.MaxWalkSpeed` (`self.MaxWalkSpeed`) (`self.CharacterMovement`)))

(event `self.ReceiveAnyDamage`
  (params (Damage :type "Float (single-precision)") (DamageType :type "DamageType Object Reference") (InstigatedBy :type "Controller Object Reference") (DamageCauser :type "Actor Object Reference"))
  (bind _output_get (set `self.HP` (- (`self.HP`) Damage)))
  (if (<= _output_get 0.0)
    (`self.K2_DestroyActor`)))

(event `self.ReceiveTick`
  (params (DeltaSeconds :type "Float (single-precision)"))
  (`KismetSystemLibrary.PrintString` (`KismetStringLibrary.Concat_StrStr` (`KismetSystemLibrary.GetDisplayName` self) " = " (`KismetStringLibrary.Conv_DoubleToString` (`self.HP`))) true true (struct :`G` 0.66 :`B` 1.0 :`A` 1.0) 0.0))

(fn `UserConstructionScript`)